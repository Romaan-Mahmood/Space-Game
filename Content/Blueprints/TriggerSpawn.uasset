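; TriggerSpawn is a trigger actor that spawns enemies when a Normal actor overlaps it while SpaceGameMode is active.
; It loops over all its child actors, using arrow and FastArrow children as spawn markers for Enemy and FastE respectively, at each marker's world location and rotation.
; Nothing disables the trigger afterwards, so each qualifying overlap spawns another set.
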(event `self.ReceiveActorBeginOverlap`
  (params (OtherActor :type "Actor Object Reference"))
  (cast `/Game/Blueprints/Player/Normal` OtherActor)
  (cast `/Game/Blueprints/SpaceGameMode` (`GameplayStatics.GetGameMode`))
  (for _array_element (`self.GetAllChildActors` true)
    (cast `/Game/Blueprints/arrow` _array_element
      (:`then`
        (bind _returnvalue (`SceneComponent.K2_GetComponentLocation` (`Actor.RootComponent` _array_element)))
        (bind _returnvalue_2 (`SceneComponent.K2_GetComponentRotation` (`Actor.RootComponent` _array_element)))
        (`|SpawnActorFromClass` "/Game/Blueprints/Enemy.Enemy_C" (`KismetMathLibrary.MakeTransform` _returnvalue _returnvalue_2) "Undefined" "MultiplyWithRoot" null null))
      (:`CastFailed`
        (cast `/Game/Blueprints/FastArrow` _array_element)
        (`|SpawnActorFromClass` "/Game/Blueprints/FastE.FastE_C" (`KismetMathLibrary.MakeTransform` _returnvalue _returnvalue_2) "Undefined" "MultiplyWithRoot" null null)))))

(fn `UserConstructionScript`)