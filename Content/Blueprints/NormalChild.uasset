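; Player-controlled pawn spawned as a child actor of the plane, handling Enhanced Input and forward flight for a space shooter.
; Each tick it sets the Base's physics velocity from speed plus move input, drags a despawner behind it and passes its transform to the plane.
; Rotation, shooting, rapid fire and detonation input forward to the parent plane.
; Boost raises speed for a limited time, then enforces a cooldown shown on the game mode's meter.
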(event `EnhancedInput|/Game/Input/Move`
  (params (ActionValue :type "Vector2D Structure") (ElapsedSeconds :type "Float (double-precision)") (TriggeredSeconds :type "Float (double-precision)") (InputAction :type "InputAction Object Reference" :default "/Game/Input/Move.Move"))
  (bind _returnvalue (`self.GetParentActor`))
  ;[1 1 1] Vertical Rotation
  (:`Triggered`
    (bind _asplane (cast `/Game/Blueprints/Player/plane` _returnvalue))
    (`/Game/Blueprints/Player/plane.VRotate` _asplane ActionValue))
  (:`Completed`
    (bind _asplane_2 (cast `/Game/Blueprints/Player/plane` _returnvalue))
    (`/Game/Blueprints/Player/plane.Stop VRotate` _asplane_2)))

(event `EnhancedInput|/Game/Input/Move`
  (params (ActionValue :type "Vector2D Structure") (ElapsedSeconds :type "Float (double-precision)") (TriggeredSeconds :type "Float (double-precision)") (InputAction :type "InputAction Object Reference" :default "/Game/Input/Move.Move"))
  (bind _returnvalue (`self.GetParentActor`))
  ;[1 1 1] Horizontal rotation
  (:`Triggered`
    (bind _asplane (cast `/Game/Blueprints/Player/plane` _returnvalue))
    (`/Game/Blueprints/Player/plane.HRotate` _asplane ActionValue))
  (:`Completed`
    (bind _asplane_2 (cast `/Game/Blueprints/Player/plane` _returnvalue))
    (`/Game/Blueprints/Player/plane.Stop HRotate` _asplane_2)))

(event `self.ReceiveBeginPlay`
  ;[1 1 1] Initialisation
  ;;[1 1 1] Add Enhanced Input
  (`GameplayStatics.SetPlayerControllerID` null)
  (bind _asplayer_controller (cast `PlayerController` (`self.GetController`)))
  (`EnhancedInputSubsystemInterface.AddMappingContext` (pcsubsystem `EnhancedInputLocalPlayerSubsystem` _asplayer_controller) "/Game/Input/Combine.Combine" 0 (struct)))

(event `EnhancedInput|/Game/Input/Move`
  (params (ActionValue :type "Vector2D Structure") (ElapsedSeconds :type "Float (double-precision)") (TriggeredSeconds :type "Float (double-precision)") (InputAction :type "InputAction Object Reference" :default "/Game/Input/Move.Move"))
  ;[1 1 1] Horizontal Movement
  (:`Triggered`
    (set `self.currentVel` (+ (`KismetMathLibrary.MakeVector` 0.0 (`KismetMathLibrary.MapRangeClamped` (.x (`KismetMathLibrary.Conv_Vector2DToVector` ActionValue)) -1.0 1.0 -4000.0 4000.0)) (`self.currentVel`)))))

(event `EnhancedInput|/Game/Input/Move`
  (params (ActionValue :type "Vector2D Structure") (ElapsedSeconds :type "Float (double-precision)") (TriggeredSeconds :type "Float (double-precision)") (InputAction :type "InputAction Object Reference" :default "/Game/Input/Move.Move"))
  ;[1 1 1] Vertical Movement
  (:`Triggered`
    (set `self.currentVel` (+ (`KismetMathLibrary.MakeVector` 0.0 0.0 (`KismetMathLibrary.MapRangeClamped` (.y (`KismetMathLibrary.Conv_Vector2DToVector` ActionValue)) -1.0 1.0 -4000.0 4000.0)) (`self.currentVel`)))))

(event `self.ReceiveTick`
  (params (DeltaSeconds :type "Float (single-precision)"))
  (bind (_returnvalue_x _returnvalue_y _returnvalue_z) (`KismetMathLibrary.BreakVector` (`SceneComponent.K2_GetComponentLocation` (`self.ChildActor`))))
  (bind _returnvalue_x_2 (`KismetMathLibrary.BreakVector` (`SceneComponent.K2_GetComponentLocation` (`self.Base`))))
  (`/Engine/EditorBlueprintResources/StandardMacros.IsValid` (`self.GetParentActor`)
    (:`Is Valid`
      ;[1 1 1] Speed
      (`PrimitiveComponent.SetPhysicsLinearVelocity` (`self.Base`) (+ (`SceneComponent.GetForwardVector` (`self.Base`)) (`self.currentVel`)) false "None")
      (set `self.currentVel` (`KismetMathLibrary.MakeVector` (`self.Speed`)))
      ;[1 1 1] Despawner Location
      (`SceneComponent.K2_SetWorldLocation` (`self.ChildActor`) (`KismetMathLibrary.MakeVector` (- _returnvalue_x_2 3000.0) _returnvalue_y _returnvalue_z) false false)
      ;[1 1 1] Pass in transform to child actor
      (bind _asplane (cast `/Game/Blueprints/Player/plane` (`self.GetParentActor`)))
      (`/Game/Blueprints/Player/plane.Set parent rot` _asplane (`SceneComponent.K2_GetComponentToWorld` (`self.Base`)))
      ;[1 1 1] Boost UI config
      (bind _asspace_game_mode (cast `/Game/Blueprints/SpaceGameMode` (`GameplayStatics.GetGameMode`)))
      (`/Game/Blueprints/SpaceGameMode.Raise Meter` _asspace_game_mode (`self.Wait`))
      (if (`self.no boost`)
        (set `self.Wait` (- (`self.Wait`) (`GameplayStatics.GetWorldDeltaSeconds`)))))
    (:`Is Not Valid`
      (`self.K2_DestroyActor`))))

(event `EnhancedInput|/Game/Input/Shoot`
  (params (ActionValue :type Boolean) (ElapsedSeconds :type "Float (double-precision)") (TriggeredSeconds :type "Float (double-precision)") (InputAction :type "InputAction Object Reference" :default "/Game/Input/Shoot.Shoot"))
  (bind _returnvalue (`self.GetParentActor`))
  (bind _returnvalue_2 (`SceneComponent.K2_GetComponentLocation` (`self.Base`)))
  ;[1 1 1] Shoot
  (:`Triggered`
    (bind _asplane (cast `/Game/Blueprints/Player/plane` _returnvalue))
    (`/Game/Blueprints/Player/plane.Charge` _asplane TriggeredSeconds))
  (:`Started`
    (bind _asplane_2 (cast `/Game/Blueprints/Player/plane` _returnvalue))
    (`/Game/Blueprints/Player/plane.Shoot` _asplane_2 _returnvalue_2))
  (:`Completed`
    (bind _asplane_3 (cast `/Game/Blueprints/Player/plane` _returnvalue))
    (`/Game/Blueprints/Player/plane.Stop charge` _asplane_3 _returnvalue_2)))

(event `EnhancedInput|/Game/Input/Rapid`
  (params (ActionValue :type "Float (double-precision)") (ElapsedSeconds :type "Float (double-precision)") (TriggeredSeconds :type "Float (double-precision)") (InputAction :type "InputAction Object Reference" :default "/Game/Input/Rapid.Rapid"))
  (bind _returnvalue (`self.GetParentActor`))
  (bind _returnvalue_2 (`SceneComponent.K2_GetComponentLocation` (`self.Base`)))
  ;[1 1 1] Shoot
  (:`Triggered`
    (bind _asplane (cast `/Game/Blueprints/Player/plane` _returnvalue))
    (`/Game/Blueprints/Player/plane. Trigger` _asplane ActionValue TriggeredSeconds _returnvalue_2))
  (:`Started`
    (bind _asplane_2 (cast `/Game/Blueprints/Player/plane` _returnvalue))
    (`/Game/Blueprints/Player/plane.Rapid Start` _asplane_2 _returnvalue_2))
  (:`Completed`
    (bind _asplane_3 (cast `/Game/Blueprints/Player/plane` _returnvalue))
    (`/Game/Blueprints/Player/plane.Rapid End` _asplane_3)))

(event `EnhancedInput|/Game/Input/Detonate`
  (params (ActionValue :type Boolean) (ElapsedSeconds :type "Float (double-precision)") (TriggeredSeconds :type "Float (double-precision)") (InputAction :type "InputAction Object Reference" :default "/Game/Input/Detonate.Detonate"))
  ;[1 1 1] Shoot
  (:`Started`
    (bind _asplane (cast `/Game/Blueprints/Player/plane` (`self.GetParentActor`)))
    (`/Game/Blueprints/Player/plane.Det` _asplane)))

(event `Increase Forward Vel`
  ;[1 1 1] Boost
  (set `self.Speed` 8000.0))

(event `EnhancedInput|/Game/Input/Boost`
  (params (ActionValue :type Boolean) (ElapsedSeconds :type "Float (double-precision)") (TriggeredSeconds :type "Float (double-precision)") (InputAction :type "InputAction Object Reference" :default "/Game/Input/Boost.Boost"))
  (bind _returnvalue (- TriggeredSeconds (`self.Diff`)))
  ;[1 1 1] Boost
  (:`Triggered`
    (if (not (`self.no boost`)) :!label _label
      (set `self.Wait` _returnvalue)
      (if (and (<= _returnvalue 3.0) ActionValue)
        (`self.Increase Forward Vel`)
        (else
          (`self.Decrease Forward Vel`)
          (set `self.no boost` true)
          (`KismetSystemLibrary.Delay` (`self.Wait`))
          (set `self.no boost` false)
          (set `self.Wait` 0.0)
          (set `self.Diff` 0.0)))))
  (:`Started`
    (set `self.Diff` 0.0)
    (goto _label))
  (:`Completed`
    (goto _label)))

(event `Decrease Forward Vel`
  ;[1 1 1] Boost
  (set `self.Speed` 4000.0))

(fn `UserConstructionScript`)