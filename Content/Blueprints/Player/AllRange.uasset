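; Player pawn for all-range space flight, driving a physics Cube forward with stick-controlled vertical velocity and yaw.
; A child plane actor receives the Cube's transform plus rotation, somersault and weapon input, and the pawn destroys itself when that child is gone.
; Timed boost switches speed, locks out while recharging, and feeds the game mode's meter.
; Once Start is set, the camera glides through four cutscene points before input is enabled.
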(event `EnhancedInput|/Game/Input/Move`
  (params (ActionValue :type "Vector2D Structure") (ElapsedSeconds :type "Float (double-precision)") (TriggeredSeconds :type "Float (double-precision)") (InputAction :type "InputAction Object Reference" :default "/Game/Input/Move.Move"))
  (bind (_returnvalue_roll _returnvalue_pitch) (`KismetMathLibrary.BreakRotator` (`SceneComponent.K2_GetComponentRotation` (`self.Cube`))))
  (bind _y (.y (`KismetMathLibrary.Conv_Vector2DToVector` ActionValue)))
  ;[1 1 1] Unused
  (:`Triggered`
    (set `self.VTarget` (+ (`self.VTarget`) (`KismetMathLibrary.MakeVector` 0.0 0.0 (`KismetMathLibrary.MapRangeClamped` _y -1.0 1.0 (* (`self.Steering`) -1.0) (`self.Steering`)))))
    (if (and (>= _y 0.0) (<= _returnvalue_pitch 0.0))
      (set `self.Vspeed` (`self.Fast interp`))
      (elif (and (<= _y 0.0) (>= _returnvalue_pitch 0.0))
        (set `self.Vspeed` (`self.Fast interp`))
        (else
          (set `self.Vspeed` (`self.Standard interp`)))))))

(event `control`
  ;[1 1 1] Add Enhanced Input
  (`self.EnableInput` (`GameplayStatics.GetPlayerController` 0)))

(event `self.ReceiveBeginPlay`
  (bind _returnvalue (`GameplayStatics.GetPlayerController` 0))
  ;[1 1 1] Initialisation
  (`SceneComponent.K2_SetWorldLocation` (`self.Camera`) (`SceneComponent.K2_GetComponentLocation` (`self.camTarget`)) false false)
  ;[1 1 1] Add Enhanced Input
  (`Controller.Possess` _returnvalue self)
  (`self.DisableInput` _returnvalue))

(event `self.ReceiveTick`
  (params (DeltaSeconds :type "Float (single-precision)"))
  (bind _returnvalue (`GameplayStatics.GetWorldDeltaSeconds`))
  (bind _camtargloc (`self.camTargLoc`))
  (bind _returnvalue_2 (`SceneComponent.K2_GetComponentLocation` (`self.Camera`)))
  (`/Engine/EditorBlueprintResources/StandardMacros.IsValid` (`ChildActorComponent.ChildActor` (`self.Plane`))
    (:`Is Valid`
      ;[1 1 1] Speed
      (`PrimitiveComponent.SetPhysicsLinearVelocity` (`self.Cube`) (+ (* (`SceneComponent.GetForwardVector` (`self.Cube`)) (`self.Speed`)) (`KismetMathLibrary.MakeVector` 0.0 0.0 (`self.currentVel`))) false "None")
      ;[1 1 1] Reset for next Tick
      (set `self.VTarget` (45.0 0.0 0.0))
      (set `self.HTarget` (45.0 0.0 0.0))
      ;[1 1 1] Pass Transform to child
      (bind _asplane (cast `/Game/Blueprints/Player/plane` (`ChildActorComponent.ChildActor` (`self.Plane`))))
      (`/Game/Blueprints/Player/plane.Set parent rot` _asplane (`SceneComponent.K2_GetComponentToWorld` (`self.Cube`)))
      ;[1 1 1] Boost UI config
      (bind _asspace_game_mode (cast `/Game/Blueprints/SpaceGameMode` (`GameplayStatics.GetGameMode`)))
      (`/Game/Blueprints/SpaceGameMode.Raise Meter` _asspace_game_mode (`self.Wait`))
      (if (`self.no boost`)
        (set `self.Wait` (- (`self.Wait`) (`GameplayStatics.GetWorldDeltaSeconds`))))
      (if (`self.start`)
        ;[1 1 1] Cutscene
        (if (`self.point1`)
          (if (`self.point2`)
            (if (`self.point3`)
              (set `self.camTargLoc` (`SceneComponent.K2_GetComponentLocation` (`self.camTarget4`)))
              (else
                (set `self.camTargLoc` (`SceneComponent.K2_GetComponentLocation` (`self.camTarget3`)))))
            (else
              (set `self.camTargLoc` (`SceneComponent.K2_GetComponentLocation` (`self.camTarget2`)))))
          (else
            (set `self.camTargLoc` (`SceneComponent.K2_GetComponentLocation` (`self.camTarget1`)))))
        (`SceneComponent.K2_SetWorldLocationAndRotation` (`self.Camera`) (`KismetMathLibrary.VInterpTo_Constant` _returnvalue_2 _camtargloc _returnvalue 1000.0) (`KismetMathLibrary.RInterpTo_Constant` (`SceneComponent.K2_GetComponentRotation` (`self.Camera`)) (`KismetMathLibrary.FindLookAtRotation` _returnvalue_2 (`SceneComponent.K2_GetComponentLocation` (`self.plane`))) _returnvalue) false false)
        (if (== _returnvalue_2 _camtargloc :`ErrorTolerance` 10.0)
          (if (`self.point1`)
            (if (`self.point2`)
              (if (`self.point3`)
                (set `self.point4` true)
                (`self.control`)
                (else
                  (set `self.point3` true)))
              (else
                (set `self.point2` true)))
            (else
              (set `self.point1` true))))))
    (:`Is Not Valid`
      (`self.K2_DestroyActor`))))

(event `EnhancedInput|/Game/Input/Move`
  (params (ActionValue :type "Vector2D Structure") (ElapsedSeconds :type "Float (double-precision)") (TriggeredSeconds :type "Float (double-precision)") (InputAction :type "InputAction Object Reference" :default "/Game/Input/Move.Move"))
  (bind _uvelocity (`self.UVelocity`))
  ;[1 1 1] Vertical Velocity
  (:`Triggered`
    (set `self.currentVel` (`KismetMathLibrary.MapRangeClamped` (.y (`KismetMathLibrary.Conv_Vector2DToVector` ActionValue)) -1.0 1.0 (* -1.0 _uvelocity) _uvelocity)))
  (:`Completed`
    (set `self.currentVel` 0.0)))

(event `EnhancedInput|/Game/Input/Move`
  (params (ActionValue :type "Vector2D Structure") (ElapsedSeconds :type "Float (double-precision)") (TriggeredSeconds :type "Float (double-precision)") (InputAction :type "InputAction Object Reference" :default "/Game/Input/Move.Move"))
  ;[1 1 1] Vertical Rotation
  (:`Triggered`
    (bind _asplane (cast `/Game/Blueprints/Player/plane` (`ChildActorComponent.ChildActor` (`self.Plane`))))
    (`/Game/Blueprints/Player/plane.VRotate` _asplane ActionValue))
  (:`Completed`
    (bind _asplane_2 (cast `/Game/Blueprints/Player/plane` (`ChildActorComponent.ChildActor` (`self.Plane`))))
    (`/Game/Blueprints/Player/plane.Stop VRotate` _asplane_2)))

(event `EnhancedInput|/Game/Input/Boost`
  (params (ActionValue :type Boolean) (ElapsedSeconds :type "Float (double-precision)") (TriggeredSeconds :type "Float (double-precision)") (InputAction :type "InputAction Object Reference" :default "/Game/Input/Boost.Boost"))
  (bind _returnvalue (- TriggeredSeconds (`self.Diff`)))
  ;[1 1 1] Boost
  (:`Triggered`
    (if (not (`self.no boost`)) :!label _label
      (set `self.Wait` _returnvalue)
      (if (and (<= _returnvalue 3.0) ActionValue)
        (`self.Increase Forward Vel`)
        (else
          (`self.Decrease Forward Vel`)
          (set `self.no boost` true)
          (`KismetSystemLibrary.Delay` (`self.Wait`))
          (set `self.no boost` false)
          (set `self.Wait` 0.0)
          (set `self.Diff` TriggeredSeconds)))))
  (:`Started`
    (set `self.Diff` 0.0)
    (goto _label))
  (:`Completed`
    (goto _label)))

(event `EnhancedInput|/Game/Input/Somersault`
  (params (ActionValue :type Boolean) (ElapsedSeconds :type "Float (double-precision)") (TriggeredSeconds :type "Float (double-precision)") (InputAction :type "InputAction Object Reference" :default "/Game/Input/Somersault.Somersault"))
  (:`Triggered`
    (bind _asplane (cast `/Game/Blueprints/Player/plane` (`ChildActorComponent.ChildActor` (`self.Plane`))))
    (`/Game/Blueprints/Player/plane.Loop` _asplane)))

(event `Increase Forward Vel`
  ;[1 1 1] Boost
  (set `self.Speed` 6000.0))

(event `Decrease Forward Vel`
  ;[1 1 1] Boost
  (set `self.Speed` 3000.0))

(event `EnhancedInput|/Game/Input/Move`
  (params (ActionValue :type "Vector2D Structure") (ElapsedSeconds :type "Float (double-precision)") (TriggeredSeconds :type "Float (double-precision)") (InputAction :type "InputAction Object Reference" :default "/Game/Input/Move.Move"))
  (bind _steering (`self.Steering`))
  ;[1 1 1] Horizontal Rotation
  (:`Triggered`
    (`SceneComponent.K2_AddLocalRotation` (`self.Cube`) (`KismetMathLibrary.MakeRotator` 0.0 0.0 (`KismetMathLibrary.MapRangeClamped` (.x (`KismetMathLibrary.Conv_Vector2DToVector` ActionValue)) -1.0 1.0 (* _steering -1.0) _steering)) false false)))

(event `EnhancedInput|/Game/Input/Shoot`
  (params (ActionValue :type Boolean) (ElapsedSeconds :type "Float (double-precision)") (TriggeredSeconds :type "Float (double-precision)") (InputAction :type "InputAction Object Reference" :default "/Game/Input/Shoot.Shoot"))
  (bind _returnvalue (`SceneComponent.K2_GetComponentLocation` (`self.Cube`)))
  ;[1 1 1] Shoot
  (:`Triggered`
    (bind _asplane (cast `/Game/Blueprints/Player/plane` (`ChildActorComponent.ChildActor` (`self.Plane`))))
    (`/Game/Blueprints/Player/plane.Charge` _asplane TriggeredSeconds))
  (:`Started`
    (bind _asplane_2 (cast `/Game/Blueprints/Player/plane` (`ChildActorComponent.ChildActor` (`self.Plane`))))
    (`/Game/Blueprints/Player/plane.Shoot` _asplane_2 _returnvalue))
  (:`Completed`
    (bind _asplane_3 (cast `/Game/Blueprints/Player/plane` (`ChildActorComponent.ChildActor` (`self.Plane`))))
    (`/Game/Blueprints/Player/plane.Stop charge` _asplane_3 _returnvalue)))

(event `EnhancedInput|/Game/Input/Move`
  (params (ActionValue :type "Vector2D Structure") (ElapsedSeconds :type "Float (double-precision)") (TriggeredSeconds :type "Float (double-precision)") (InputAction :type "InputAction Object Reference" :default "/Game/Input/Move.Move"))
  ;[1 1 1] Horizontal Rotation
  (:`Triggered`
    (bind _asplane (cast `/Game/Blueprints/Player/plane` (`ChildActorComponent.ChildActor` (`self.Plane`))))
    (`/Game/Blueprints/Player/plane.HRotate` _asplane ActionValue))
  (:`Completed`
    (bind _asplane_2 (cast `/Game/Blueprints/Player/plane` (`ChildActorComponent.ChildActor` (`self.Plane`))))
    (`/Game/Blueprints/Player/plane.Stop HRotate` _asplane_2)))

(event `EnhancedInput|/Game/Input/Rapid`
  (params (ActionValue :type "Float (double-precision)") (ElapsedSeconds :type "Float (double-precision)") (TriggeredSeconds :type "Float (double-precision)") (InputAction :type "InputAction Object Reference" :default "/Game/Input/Rapid.Rapid"))
  (bind _returnvalue (`SceneComponent.K2_GetComponentLocation` (`self.Cube`)))
  (bind _childactor (`ChildActorComponent.ChildActor` (`self.Plane`)))
  ;[1 1 1] Shoot
  (:`Triggered`
    (bind _asplane (cast `/Game/Blueprints/Player/plane` _childactor))
    (`/Game/Blueprints/Player/plane. Trigger` _asplane ActionValue TriggeredSeconds _returnvalue))
  (:`Started`
    (bind _asplane_2 (cast `/Game/Blueprints/Player/plane` _childactor))
    (`/Game/Blueprints/Player/plane.Rapid Start` _asplane_2 _returnvalue))
  (:`Completed`
    (bind _asplane_3 (cast `/Game/Blueprints/Player/plane` _childactor))
    (`/Game/Blueprints/Player/plane.Rapid End` _asplane_3)))

(event `EnhancedInput|/Game/Input/Detonate`
  (params (ActionValue :type Boolean) (ElapsedSeconds :type "Float (double-precision)") (TriggeredSeconds :type "Float (double-precision)") (InputAction :type "InputAction Object Reference" :default "/Game/Input/Detonate.Detonate"))
  ;[1 1 1] Shoot
  (:`Started`
    (bind _asplane (cast `/Game/Blueprints/Player/plane` (`ChildActorComponent.ChildActor` (`self.Plane`))))
    (`/Game/Blueprints/Player/plane.Det` _asplane)))

(fn `UserConstructionScript`)