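; Player charge-shot projectile that flies forward and explodes when Detonate is called or 0.8 seconds after spawning.
; Tick drives BigLaser's physics velocity along its forward vector until detonation stops it.
; Detonation spawns a large explosion and briefly enlarges Box before destroying the actor.
; Bshot calls accumulate a Bonus counter, which is sent to SpaceGameMode as score, less one, just before destruction.
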(event `Detonate`
  (bind _bonus (`self.bonus`))
  ;[1 1 1] Destroy Conditions
  (`GameplayStatics.SpawnEmitterAtLocation` "/Game/StarterContent/Particles/P_Explosion.P_Explosion" (`SceneComponent.K2_GetComponentLocation` (`self.Big laser`)) (struct) (10.0 10.0 10.0) :!label _label)
  (set `self.destroyed` true)
  (`SceneComponent.SetRelativeScale3D` (`self.Box`) (20.0 10.0 10.0))
  (`KismetSystemLibrary.Delay` 0.2)
  (bind _asspace_game_mode (cast `/Game/Blueprints/SpaceGameMode` (`GameplayStatics.GetGameMode`)))
  (if (== _bonus 0)
    (`/Game/Blueprints/SpaceGameMode.Add Score` _asspace_game_mode 0)
    (else
      (`/Game/Blueprints/SpaceGameMode.Add Score` _asspace_game_mode (- _bonus 1))))
  (`self.K2_DestroyActor`))

(event `Bshot`
  ;[1 1 1] Destroy Conditions
  (set `self.bonus` (+ (`self.bonus`) 1)))

(event `self.ReceiveBeginPlay`
  ;[1 1 1] Destroy Conditions
  (`KismetSystemLibrary.Delay` 0.8)
  (goto _label))

(event `self.ReceiveTick`
  (params (DeltaSeconds :type "Float (single-precision)"))
  ;[1 1 1] Speed
  (if (`self.destroyed`)
    (`PrimitiveComponent.SetPhysicsLinearVelocity` (`self.Big laser`) (0.0 0.0 0.0) false "None")
    (else
      (`PrimitiveComponent.SetPhysicsLinearVelocity` (`self.Big laser`) (* (`SceneComponent.GetForwardVector` (`self.Big laser`)) (`self.Speed`)) false "None"))))

(fn `UserConstructionScript`)