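; Parent Blueprint for the player's plane, handling steering, weapons and damage.
; Steering inputs set per-tick targets that Tick interpolates Base toward, yaw relative to a supplied parent transform and roll zeroed, turning faster when returning to center.
; Weapons include rapid fire paced by trigger pressure and a detonatable charge shot that blocks normal fire while charging.
; Non-excluded overlaps cost health via SpaceGameMode, with brief invulnerability, then explosion at zero.
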(event `HRotate`
  (params (`Input Value` :type "Vector2D Structure"))
  (bind (_returnvalue_roll _returnvalue_pitch _returnvalue_yaw) (`KismetMathLibrary.BreakRotator` (`KismetMathLibrary.FindRelativeLookAtRotation` (`self.Parent transform`) (`SceneComponent.K2_GetComponentLocation` (`self.Cube`)))))
  ;[1 1 1] Horizontal Rotation
  (set `self.HVector` (.x (`KismetMathLibrary.Conv_Vector2DToVector` `Input Value`)))
  (set `self.HTarget` (+ (`self.HTarget`) (`KismetMathLibrary.MakeVector` 0.0 (`KismetMathLibrary.MapRangeClamped` (`self.HVector`) -1.0 1.0 -45.0 45.0))))
  (if (and (<= (`self.HVector`) 0.0) (>= _returnvalue_yaw 0.0)) :!label _label
    (set `self.HSpeed` (`self.Fast interp`))
    (elif (and (<= _returnvalue_yaw 0.0) (>= (`self.HVector`) 0.0))
      (set `self.HSpeed` (`self.Fast interp`))
      (else
        (set `self.HSpeed` (`self.Standard interp`))))))

(event `VRotate`
  (params (`Input Value` :type "Vector2D Structure"))
  (bind (_returnvalue_roll _returnvalue_pitch) (`KismetMathLibrary.BreakRotator` (`SceneComponent.K2_GetComponentRotation` (`self.Base`))))
  (bind _y (.y (`KismetMathLibrary.Conv_Vector2DToVector` `Input Value`)))
  ;[1 1 1] Vertical Rotation
  (set `self.VTarget` (+ (`self.VTarget`) (`KismetMathLibrary.MakeVector` 0.0 0.0 (`KismetMathLibrary.MapRangeClamped` _y -1.0 1.0 -45.0 45.0))))
  (if (and (>= _y 0.0) (<= _returnvalue_pitch 0.0)) :!label _label_2
    (set `self.Vspeed` (`self.Fast interp`))
    (elif (and (<= _y 0.0) (>= _returnvalue_pitch 0.0))
      (set `self.Vspeed` (`self.Fast interp`))
      (else
        (set `self.Vspeed` (`self.Standard interp`))))))

(event `Stop VRotate`
  ;[1 1 1] Vertical Rotation
  (goto _label_2))

(event `Stop HRotate`
  ;[1 1 1] Horizontal Rotation
  (set `self.HVector` 0.0)
  (goto _label))

(event `Set parent rot`
  (params (NewParam :type "Transform Structure"))
  (set `self.Parent transform` NewParam))

(event `Det`
  (`/Game/Blueprints/Player/ChargeShotP.Detonate` (stale `Stop charge` _returnvalue)))

(event `Stop charge`
  (params (`Shoot Loc` :type "Vector Structure"))
  ;[1 1 1] Shoot
  (set `self.Charging` false)
  (if (`self.Charged`)
    (set `self.Charged` false)
    (bind _returnvalue (`|SpawnActorFromClass` "/Game/Blueprints/Player/ChargeShotP.ChargeShotP_C" (`KismetMathLibrary.MakeTransform` `Shoot Loc` (`SceneComponent.K2_GetComponentRotation` (`self.Base`))) "AlwaysSpawn" "MultiplyWithRoot" null null))))

(event `self.ReceiveTick`
  (params (DeltaSeconds :type "Float (single-precision)"))
  (bind (_returnvalue_roll _returnvalue_pitch _returnvalue_yaw) (`KismetMathLibrary.BreakRotator` (`SceneComponent.K2_GetComponentRotation` (`self.base`))))
  (bind (_returnvalue_roll_2 _returnvalue_pitch_2 _returnvalue_yaw_2) (`KismetMathLibrary.BreakRotator` (`KismetMathLibrary.FindRelativeLookAtRotation` (`self.Parent transform`) (`SceneComponent.K2_GetComponentLocation` (`self.Cube`)))))
  (bind (_returnvalue_roll_3 _returnvalue_pitch_3 _returnvalue_yaw_3) (`KismetMathLibrary.BreakRotator` (`KismetMathLibrary.NormalizedDeltaRotator` (`KismetMathLibrary.Conv_VectorToRotator` (`self.HTarget`)) (`KismetMathLibrary.MakeRotator` 0.0 0.0 _returnvalue_yaw_2))))
  (bind (_returnvalue_roll_4 _returnvalue_pitch_4) (`KismetMathLibrary.BreakRotator` (`KismetMathLibrary.RInterpTo` (struct) (`KismetMathLibrary.NormalizedDeltaRotator` (`KismetMathLibrary.Conv_VectorToRotator` (`self.VTarget`)) (`SceneComponent.K2_GetComponentRotation` (`self.base`))) (`GameplayStatics.GetWorldDeltaSeconds`) (`self.Vspeed`))))
  ;[1 1 1] Universal rotation interpolator
  ;;[1 1 1] Horizontal
  (`SceneComponent.K2_AddLocalRotation` (`self.Base`) (`KismetMathLibrary.RInterpTo` (struct) (`KismetMathLibrary.MakeRotator` 0.0 0.0 _returnvalue_yaw_3) DeltaSeconds (`self.HSpeed`)) false false)
  ;;[1 1 1] Vertical
  (`SceneComponent.K2_AddLocalRotation` (`self.Base`) (`KismetMathLibrary.MakeRotator` 0.0 _returnvalue_pitch_4) false false)
  ;[1 1 1] Reset for next Tick
  (set `self.HTarget` (45.0 0.0 0.0))
  (set `self.VTarget` (45.0 0.0 0.0))
  (`SceneComponent.K2_SetWorldRotation` (`self.base`) (`KismetMathLibrary.MakeRotator` 0.0 _returnvalue_pitch _returnvalue_yaw) false false))

(event `Charge`
  (params (Time :type "Float (double-precision)"))
  ;[1 1 1] Shoot
  (set `self.Charging` true)
  (if (>= Time 1.0)
    (bind _output_get (set `self.Charged` true))
    (`KismetSystemLibrary.PrintText` (`KismetTextLibrary.Conv_BoolToText` _output_get))))

(event `Shoot`
  (params (`Shoot Loc` :type "Vector Structure"))
  ;[1 1 1] Shoot
  (`|SpawnActorFromClass` "/Game/Blueprints/Player/Bullet.Bullet_C" (`KismetMathLibrary.MakeTransform` `Shoot Loc` (`SceneComponent.K2_GetComponentRotation` (`self.Base`))) "AlwaysSpawn" "MultiplyWithRoot" null null))

(event `Trigger`
  (params (`Input Value` :type "Float (double-precision)") (Time :type "Float (double-precision)") (`Shoot Loc` :type "Vector Structure"))
  ;[1 1 1] Rapid Fire
  (if (`self.Charging`)
    _
    (elif (>= (- Time (`self.rapidTime`)) (`KismetMathLibrary.MapRangeClamped` `Input Value` 0.0 1.0 0.7 0.1))
      (set `self.rapidTime` Time)
      (if (`self.Rapid`)
        (`self.Shoot` `Shoot Loc`)))))

(event `Rapid End`
  ;[1 1 1] Rapid Fire
  (set `self.Rapid` false))

(event `Rapid Start`
  (params (`Shoot Loc` :type "Vector Structure"))
  ;[1 1 1] Rapid Fire
  (set `self.rapidTime` 0.0)
  (set `self.Rapid` true)
  (if (not (`self.Charging`))
    (`self.Shoot` `Shoot Loc`)))

(event `self.ReceiveActorBeginOverlap`
  (params (OtherActor :type "Actor Object Reference"))
  ;[1 1 1] When Hit
  (cast `/Game/Blueprints/Player/Bullet` OtherActor
    (:`CastFailed`
      (cast `/Game/Blueprints/TriggerSpawn` OtherActor
        (:`CastFailed`
          (cast `/Game/Blueprints/Player/ChargeShotP` OtherActor
            (:`CastFailed`
              (cast `/Game/Blueprints/Despawner` OtherActor
                (:`CastFailed`
                  (if (`self.canBeDam`)
                    (bind _asspace_game_mode (cast `/Game/Blueprints/SpaceGameMode` (`GameplayStatics.GetGameMode`)))
                    (`/Game/Blueprints/SpaceGameMode.Lose Health` _asspace_game_mode)
                    (set `self.canBeDam` false)
                    (bind _output_get (set `self.health` (- (`self.health`) 1)))
                    (bind _returnvalue (> _output_get 0))
                    (if _returnvalue
                      (`KismetSystemLibrary.Delay` 0.5)
                      (else
                        (`self.DisableInput` null)))
                    (if _returnvalue
                      (set `self.canBeDam` true)
                      (else
                        (`GameplayStatics.SpawnEmitterAtLocation` "/Game/StarterContent/Particles/P_Explosion.P_Explosion" (`SceneComponent.K2_GetComponentLocation` (`self.Base`)) (struct) (10.0 10.0 10.0))
                        (`self.K2_DestroyActor`)))))))))))))

(fn `UserConstructionScript`)