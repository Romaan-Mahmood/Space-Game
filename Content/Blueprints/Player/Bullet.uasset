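; Player projectile Blueprint that flies forward and destroys itself on impact or after a short lifetime.
; Each Tick overwrites the Laser component's physics linear velocity with the root's forward vector scaled by Speed.
; A chain of casts on overlap exempts other bullets, Ship, TriggerSpawn, plane, Normal and DespawnPlayer actors; any other actor triggers destruction.
; A BeginPlay delay feeds the same destroy call, capping the bullet's lifetime.
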(event `self.ReceiveActorBeginOverlap`
  (params (OtherActor :type "Actor Object Reference"))
  ;[1 1 1] Destroy Conditions
  (cast `/Game/Blueprints/Player/Bullet` OtherActor
    (:`CastFailed`
      (cast `/Game/Blueprints/Player/Ship` OtherActor
        (:`CastFailed`
          (cast `/Game/Blueprints/TriggerSpawn` OtherActor
            (:`CastFailed`
              (cast `/Game/Blueprints/Player/plane` OtherActor
                (:`CastFailed`
                  (cast `/Game/Blueprints/Player/Normal` OtherActor
                    (:`CastFailed`
                      (cast `/Game/Blueprints/DespawnPlayer` OtherActor
                        (:`CastFailed`
                          (`self.K2_DestroyActor` :!label _label))))))))))))))

(event `self.ReceiveBeginPlay`
  ;[1 1 1] Destroy Conditions
  (`KismetSystemLibrary.Delay` 0.8)
  (goto _label))

(event `self.ReceiveTick`
  (params (DeltaSeconds :type "Float (single-precision)"))
  ;[1 1 1] Speed
  (`PrimitiveComponent.SetPhysicsLinearVelocity` (`self.Laser`) (* (`SceneComponent.GetForwardVector` (`self.DefaultSceneRoot`)) (`self.Speed`)) false "None"))

(fn `UserConstructionScript`)