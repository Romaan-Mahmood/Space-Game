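; Player ship pawn for a space shooter: flies constantly along +X, with steering, shooting, timed boost and damage handling.
; Enhanced Input feeds rotation targets and velocity, which Tick applies via RInterpTo and physics velocity, then resets, while repositioning a trailing despawner.
; Weapons include bullets, detonatable charge shots and analog-rate rapid fire.
; Boost and hits report to SpaceGameMode; old key controls, unfinished rolls and disconnected meter logic remain.
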(event `self.ReceiveBeginPlay`
  ;[1 1 1] Initialisation
  ;;[1 1 1] Add Enhanced Input
  (bind _asplayer_controller (cast `PlayerController` (`self.GetController`)))
  (`EnhancedInputSubsystemInterface.AddMappingContext` (pcsubsystem `EnhancedInputLocalPlayerSubsystem` _asplayer_controller) "/Game/Input/Combine.Combine" 0 (struct)))

(event `Key|Up`
  (params (Key :type "Key Structure"))
  (bind _currentvel (`self.currentVel`))
  (bind _verticalspeed (`self.verticalSpeed`))
  ;[1 1 1] Old
  ;;[1 1 1] Moving Up
  (:`Pressed`
    (set `self.HTarget` (+ (`self.HTarget`) (`self.upAdd`)))
    (set `self.currentVel` (+ _verticalspeed _currentvel))
    (set `self.up` true))
  (:`Released`
    (set `self.HTarget` (+ (`self.HTarget`) (`self.upMinus`)))
    (set `self.currentVel` (- _currentvel _verticalspeed))
    (set `self.up` false)))

(event `Key|Down`
  (params (Key :type "Key Structure"))
  (bind _currentvel (`self.currentVel`))
  (bind _verticalspeed (`self.verticalSpeed`))
  ;[1 1 1] Old
  ;;[1 1 1] Moving Down
  (:`Pressed`
    (set `self.HTarget` (+ (`self.HTarget`) (`self.upMinus`)))
    (set `self.currentVel` (- _currentvel _verticalspeed))
    (set `self.down` true))
  (:`Released`
    (set `self.HTarget` (+ (`self.HTarget`) (`self.upAdd`)))
    (set `self.currentVel` (+ _verticalspeed _currentvel))
    (set `self.down` false)))

(event `EnhancedInput|/Game/Input/Move`
  (params (ActionValue :type "Vector2D Structure") (ElapsedSeconds :type "Float (double-precision)") (TriggeredSeconds :type "Float (double-precision)") (InputAction :type "InputAction Object Reference" :default "/Game/Input/Move.Move"))
  (bind (_returnvalue_roll _returnvalue_pitch _returnvalue_yaw) (`KismetMathLibrary.BreakRotator` (`SceneComponent.K2_GetComponentRotation` (`self.Base`))))
  (bind _x (.x (`KismetMathLibrary.Conv_Vector2DToVector` ActionValue)))
  ;[1 1 1] Horizontal Rotation
  (:`Triggered`
    (set `self.HTarget` (+ (`self.HTarget`) (`KismetMathLibrary.MakeVector` 0.0 (`KismetMathLibrary.MapRangeClamped` _x -1.0 1.0 -45.0 45.0))))
    (if (and (<= _x 0.0) (>= _returnvalue_yaw 0.0)) :!label _label
      (set `self.HSpeed` (`self.Fast interp`))
      (elif (and (<= _returnvalue_yaw 0.0) (>= _x 0.0))
        (set `self.HSpeed` (`self.Fast interp`))
        (else
          (set `self.HSpeed` (`self.Standard interp`))))))
  (:`Completed`
    (goto _label)))

(event `EnhancedInput|/Game/Input/Move`
  (params (ActionValue :type "Vector2D Structure") (ElapsedSeconds :type "Float (double-precision)") (TriggeredSeconds :type "Float (double-precision)") (InputAction :type "InputAction Object Reference" :default "/Game/Input/Move.Move"))
  (bind (_returnvalue_roll _returnvalue_pitch) (`KismetMathLibrary.BreakRotator` (`SceneComponent.K2_GetComponentRotation` (`self.Base`))))
  (bind _y (.y (`KismetMathLibrary.Conv_Vector2DToVector` ActionValue)))
  ;[1 1 1] Vertical Rotation
  (:`Triggered`
    (set `self.VTarget` (+ (`self.VTarget`) (`KismetMathLibrary.MakeVector` 0.0 0.0 (`KismetMathLibrary.MapRangeClamped` _y -1.0 1.0 -45.0 45.0))))
    (if (and (>= _y 0.0) (<= _returnvalue_pitch 0.0)) :!label _label_2
      (set `self.Vspeed` (`self.Fast interp`))
      (elif (and (<= _y 0.0) (>= _returnvalue_pitch 0.0))
        (set `self.Vspeed` (`self.Fast interp`))
        (else
          (set `self.Vspeed` (`self.Standard interp`))))))
  (:`Completed`
    (goto _label_2)))

(event `Key|Left`
  (params (Key :type "Key Structure"))
  (bind _currentvel (`self.currentVel`))
  (bind _horizontalspeed (`self.horizontalSpeed`))
  ;[1 1 1] Old
  ;;[1 1 1] Moving Left
  (:`Pressed`
    (set `self.HTarget` (+ (`self.HTarget`) (`self.rightMinus`)))
    (set `self.currentVel` (- _currentvel _horizontalspeed))
    (set `self.left` true))
  (:`Released`
    (set `self.HTarget` (+ (`self.HTarget`) (`self.rightAdd`)))
    (set `self.currentVel` (+ _horizontalspeed _currentvel))
    (set `self.left` false)))

(event `Key|Right`
  (params (Key :type "Key Structure"))
  (bind _currentvel (`self.currentVel`))
  (bind _horizontalspeed (`self.horizontalSpeed`))
  ;[1 1 1] Old
  ;;[1 1 1] Moving Right
  (:`Pressed`
    (set `self.HTarget` (+ (`self.HTarget`) (`self.rightAdd`)))
    (set `self.currentVel` (+ _horizontalspeed _currentvel))
    (set `self.right` true))
  (:`Released`
    (set `self.HTarget` (+ (`self.HTarget`) (`self.rightMinus`)))
    (set `self.currentVel` (- _currentvel _horizontalspeed))
    (set `self.right` false)))

(event `Key|E`
  (params (Key :type "Key Structure"))
  ;[1 1 1] Unfinished
  ;;[1 1 1] Rolling Right (Unfinished)
  (:`Pressed`
    (set `self.planeTarget` (`KismetMathLibrary.ComposeRotators` (`self.planeTarget`) (`self.rollRightAdd`))))
  (:`Released`
    (set `self.planeTarget` (`KismetMathLibrary.ComposeRotators` (`self.planeTarget`) (`self.rollRightMinus`)))))

(event `Key|Q`
  (params (Key :type "Key Structure"))
  ;[1 1 1] Unfinished
  ;;[1 1 1] Rolling Left (Unfinished)
  (:`Pressed`
    (set `self.HTarget` (0.0 0.0 0.0)))
  (:`Released`
    (set `self.HTarget` (0.0 0.0 0.0))))

(event `EnhancedInput|/Game/Input/Move`
  (params (ActionValue :type "Vector2D Structure") (ElapsedSeconds :type "Float (double-precision)") (TriggeredSeconds :type "Float (double-precision)") (InputAction :type "InputAction Object Reference" :default "/Game/Input/Move.Move"))
  ;[1 1 1] Horizontal Movement
  (:`Triggered`
    (set `self.currentVel` (+ (`KismetMathLibrary.MakeVector` 0.0 (`KismetMathLibrary.MapRangeClamped` (.x (`KismetMathLibrary.Conv_Vector2DToVector` ActionValue)) -1.0 1.0 -4000.0 4000.0)) (`self.currentVel`)))))

(event `EnhancedInput|/Game/Input/Move`
  (params (ActionValue :type "Vector2D Structure") (ElapsedSeconds :type "Float (double-precision)") (TriggeredSeconds :type "Float (double-precision)") (InputAction :type "InputAction Object Reference" :default "/Game/Input/Move.Move"))
  ;[1 1 1] Vertical Movement
  (:`Triggered`
    (set `self.currentVel` (+ (`KismetMathLibrary.MakeVector` 0.0 0.0 (`KismetMathLibrary.MapRangeClamped` (.y (`KismetMathLibrary.Conv_Vector2DToVector` ActionValue)) -1.0 1.0 -4000.0 4000.0)) (`self.currentVel`)))))

(event `EnhancedInput|/Game/Input/Detonate`
  (params (ActionValue :type Boolean) (ElapsedSeconds :type "Float (double-precision)") (TriggeredSeconds :type "Float (double-precision)") (InputAction :type "InputAction Object Reference" :default "/Game/Input/Detonate.Detonate"))
  ;[1 1 1] Spawn Bullet
  (:`Started`
    (`/Game/Blueprints/Player/ChargeShotP.Detonate` (stale `EnhancedInput|/Game/Input/Shoot` _returnvalue_3))))

(event `EnhancedInput|/Game/Input/Shoot`
  (params (ActionValue :type Boolean) (ElapsedSeconds :type "Float (double-precision)") (TriggeredSeconds :type "Float (double-precision)") (InputAction :type "InputAction Object Reference" :default "/Game/Input/Shoot.Shoot"))
  (bind _returnvalue (`SceneComponent.K2_GetComponentRotation` (`self.Base`)))
  (bind _returnvalue_2 (+ (`SceneComponent.K2_GetComponentLocation` (`self.Base`)) (1200.0 -20.0 -200.0)))
  ;[1 1 1] Spawn Bullet
  (:`Triggered`
    (set `self.Charging` true)
    (if (>= ElapsedSeconds 1.0)
      (bind _output_get (set `self.Charged` true))
      (`KismetSystemLibrary.PrintText` (`KismetTextLibrary.Conv_BoolToText` _output_get))))
  (:`Started`
    (`|SpawnActorFromClass` "/Game/Blueprints/Player/Bullet.Bullet_C" (`KismetMathLibrary.MakeTransform` _returnvalue_2 _returnvalue) "AlwaysSpawn" "MultiplyWithRoot" null null :!label _label_3))
  (:`Completed`
    (set `self.Charging` false)
    (if (`self.Charged`)
      (set `self.Charged` false)
      (bind _returnvalue_3 (`|SpawnActorFromClass` "/Game/Blueprints/Player/ChargeShotP.ChargeShotP_C" (`KismetMathLibrary.MakeTransform` _returnvalue_2 _returnvalue) "AlwaysSpawn" "MultiplyWithRoot" null null)))))

(event `EnhancedInput|/Game/Input/Rapid`
  (params (ActionValue :type "Float (double-precision)") (ElapsedSeconds :type "Float (double-precision)") (TriggeredSeconds :type "Float (double-precision)") (InputAction :type "InputAction Object Reference" :default "/Game/Input/Rapid.Rapid"))
  ;[1 1 1] Rapid Fire
  (:`Triggered`
    (if (`self.Charging`)
      _
      (elif (>= (- TriggeredSeconds (`self.rapidTime`)) (`KismetMathLibrary.MapRangeClamped` ActionValue 0.0 1.0 0.7 0.1))
        (set `self.rapidTime` TriggeredSeconds)
        (if (`self.Rapid`)
          (goto _label_3)))))
  (:`Started`
    (set `self.rapidTime` 0.0)
    (set `self.Rapid` true)
    (if (not (`self.Charging`))
      (goto _label_3)))
  (:`Completed`
    (set `self.Rapid` false)))

(event `Increase meter`
  ;[1 1 1] Old
  ;;[1 1 1] Boost
  (if (<= (`self.boostMeter`) 4.9)
    (`/Engine/EditorBlueprintResources/StandardMacros.Gate` true
      (:`Exit`
        (if (`self.loop`)
          (set `self.boostMeter` (+ (`self.boostMeter`) 0.1))
          (bind _asspace_game_mode (cast `/Game/Blueprints/SpaceGameMode` (`GameplayStatics.GetGameMode`)))
          (`/Game/Blueprints/SpaceGameMode.Raise Meter` _asspace_game_mode 0.0))))
    (else
      (`self.Decrease Forward Vel`)
      (set `self.loop` false)
      (set `self.loopCool` true))))

(event `EnhancedInput|/Game/Input/Boost`
  (params (ActionValue :type Boolean) (ElapsedSeconds :type "Float (double-precision)") (TriggeredSeconds :type "Float (double-precision)") (InputAction :type "InputAction Object Reference" :default "/Game/Input/Boost.Boost"))
  ;[1 1 1] Old
  ;;[1 1 1] Boost
)

(event `self.ReceiveTick`
  (params (DeltaSeconds :type "Float (single-precision)"))
  (bind _returnvalue_x (`KismetMathLibrary.BreakVector` (`SceneComponent.K2_GetComponentLocation` (`self.Base`))))
  (bind (_returnvalue_x_2 _returnvalue_y _returnvalue_z) (`KismetMathLibrary.BreakVector` (`SceneComponent.K2_GetComponentLocation` (`self.ChildActor`))))
  ;[1 1 1] Universal rotation interpolator
  ;;[1 1 1] Horizontal
  (`SceneComponent.K2_AddLocalRotation` (`self.Base`) (`KismetMathLibrary.RInterpTo` (struct) (`KismetMathLibrary.NormalizedDeltaRotator` (`KismetMathLibrary.Conv_VectorToRotator` (`self.HTarget`)) (`SceneComponent.K2_GetComponentRotation` (`self.Base`))) DeltaSeconds (`self.HSpeed`)) false false)
  ;;[1 1 1] Vertical
  (`SceneComponent.K2_AddLocalRotation` (`self.Base`) (`KismetMathLibrary.RInterpTo` (struct) (`KismetMathLibrary.NormalizedDeltaRotator` (`KismetMathLibrary.Conv_VectorToRotator` (`self.VTarget`)) (`SceneComponent.K2_GetComponentRotation` (`self.Base`))) (`GameplayStatics.GetWorldDeltaSeconds`) (`self.Vspeed`)) false false)
  ;[1 1 1] Set Vertical and Horizontal Speed
  (`PrimitiveComponent.SetPhysicsLinearVelocity` (`self.Base`) (`self.currentVel`) false "None")
  ;[1 1 1] Reset for next Tick
  (set `self.HTarget` (45.0 0.0 0.0))
  (set `self.VTarget` (45.0 0.0 0.0))
  (set `self.currentVel` (`KismetMathLibrary.MakeVector` (`self.Speed`)))
  ;[1 1 1] Despawner Location
  (`SceneComponent.K2_SetWorldLocation` (`self.ChildActor`) (`KismetMathLibrary.MakeVector` (- _returnvalue_x 3000.0) _returnvalue_y _returnvalue_z) false false)
  ;[1 1 1] Boost UI config
  (bind _asspace_game_mode (cast `/Game/Blueprints/SpaceGameMode` (`GameplayStatics.GetGameMode`)))
  (`/Game/Blueprints/SpaceGameMode.Raise Meter` _asspace_game_mode (`self.Wait`))
  (if (`self.no boost`)
    (set `self.Wait` (- (`self.Wait`) (`GameplayStatics.GetWorldDeltaSeconds`)))))

(event `Cooldown`
  (bind _boostmeter (`self.boostMeter`))
  ;[1 1 1] Old
  ;;[1 1 1] Meter Cooldown
  (if (<= _boostmeter 0.0)
    (set `self.loopCool` false)
    (elif (`self.loopCool`)
      (set `self.boostMeter` (- _boostmeter 0.1))
      (bind _asspace_game_mode (cast `/Game/Blueprints/SpaceGameMode` (`GameplayStatics.GetGameMode`)))
      (`/Game/Blueprints/SpaceGameMode.Lower Meter` _asspace_game_mode))))

(event `Increase Forward Vel`
  ;[1 1 1] Boost Feature
  (set `self.Speed` 8000.0))

(event `EnhancedInput|/Game/Input/Boost`
  (params (ActionValue :type Boolean) (ElapsedSeconds :type "Float (double-precision)") (TriggeredSeconds :type "Float (double-precision)") (InputAction :type "InputAction Object Reference" :default "/Game/Input/Boost.Boost"))
  (bind _returnvalue (- TriggeredSeconds (`self.Diff`)))
  ;[1 1 1] Boost Feature
  (:`Triggered`
    (if (not (`self.no boost`)) :!label _label_4
      (set `self.Wait` _returnvalue)
      (if (and (<= _returnvalue 3.0) ActionValue)
        (`self.Increase Forward Vel`)
        (else
          (`self.Decrease Forward Vel`)
          (set `self.no boost` true)
          (`KismetSystemLibrary.Delay` (`self.Wait`))
          (set `self.no boost` false)
          (set `self.Wait` 0.0)
          (set `self.Diff` TriggeredSeconds)))))
  (:`Started`
    (set `self.Diff` 0.0)
    (goto _label_4))
  (:`Completed`
    (goto _label_4)))

(event `Decrease Forward Vel`
  ;[1 1 1] Boost Feature
  (set `self.Speed` 4000.0))

(event `self.ReceiveActorBeginOverlap`
  (params (OtherActor :type "Actor Object Reference"))
  ;[1 1 1] When Hit
  (cast `/Game/Blueprints/Player/Bullet` OtherActor
    (:`CastFailed`
      (cast `/Game/Blueprints/TriggerSpawn` OtherActor
        (:`CastFailed`
          (cast `/Game/Blueprints/Player/ChargeShotP` OtherActor
            (:`CastFailed`
              (cast `/Game/Blueprints/Despawner` OtherActor
                (:`CastFailed`
                  (if (`self.canBeDam`)
                    (bind _asspace_game_mode (cast `/Game/Blueprints/SpaceGameMode` (`GameplayStatics.GetGameMode`)))
                    (`/Game/Blueprints/SpaceGameMode.Lose Health` _asspace_game_mode)
                    (set `self.canBeDam` false)
                    (bind _output_get (set `self.health` (- (`self.health`) 1)))
                    (bind _returnvalue (> _output_get 0))
                    (if _returnvalue
                      (`KismetSystemLibrary.Delay` 0.5)
                      (else
                        (`self.DisableInput` null)))
                    (if _returnvalue
                      (set `self.canBeDam` true)
                      (else
                        (`GameplayStatics.SpawnEmitterAtLocation` "/Game/StarterContent/Particles/P_Explosion.P_Explosion" (`SceneComponent.K2_GetComponentLocation` (`self.Base`)) (struct) (10.0 10.0 10.0))
                        (`self.K2_DestroyActor`)))))))))))))

(fn `UserConstructionScript`)