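; Space game mode that creates the HUD and tracks score, health and boost meter for it.
; Events add score, decrement health, and lower or set the meter, pushing each new value to the UI widget.
; getScore, despite its name, passes Health to a plane through GetHealth.
; CheckTrigger spawns an Enemy while TriggerNum is zero; the counter's increment is disconnected.
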(event `self.ReceiveBeginPlay`
  (bind _returnvalue (`|GenericCreateObject` "/Game/Blueprints/UI.UI_C"))
  (`UserWidget.AddToViewport` _returnvalue 0)
  (bind _output_get (set `self.UI` _returnvalue))
  (`/Game/Blueprints/UI.Set Score Text` _output_get 0)
  (`/Game/Blueprints/UI.Set Health Text` _output_get 3)
  (`/Game/Blueprints/UI.Set Boost Meter` _output_get 0.0))

(event `Add Score`
  (params (ScoreAdd :type Integer))
  (bind _output_get (set `self.Score` (+ ScoreAdd (`self.Score`))))
  (`/Game/Blueprints/UI.Set Score Text` (`self.UI`) _output_get))

(event `Lose Health`
  (bind _output_get (set `self.Health` (- (`self.Health`) 1)))
  (`/Game/Blueprints/UI.Set Health Text` (`self.UI`) _output_get))

(event `get Score`
  (params (Plane :type "/Game/Blueprints/Player/plane Object Reference"))
  (bind _asplane (cast `/Game/Blueprints/Player/plane` Plane))
  (`/Game/Blueprints/Player/plane.get Health` _asplane (`self.Health`)))

(event `Lower Meter`
  (bind _output_get (set `self.Meter` (- (`self.Meter`) 0.1)))
  (`/Game/Blueprints/UI.Set Boost Meter` (`self.UI`) _output_get))

(event `Raise Meter`
  (params (Time :type "Float (double-precision)"))
  (bind _output_get (set `self.Meter` Time))
  (`/Game/Blueprints/UI.Set Boost Meter` (`self.UI`) _output_get))

(event `Check Trigger`
  (if (== (`self.TriggerNum`) 0)
    (`|SpawnActorFromClass` "/Game/Blueprints/Enemy.Enemy_C" (`KismetMathLibrary.MakeTransform` (0.0 0.0 0.0)) "Undefined" "MultiplyWithRoot" null null)))

(fn `UserConstructionScript`)