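; FastE is an enemy in a space game that flies along its forward vector at Speed using physics velocity.
; It holds its spawn rotation for eight seconds, eases toward a fixed heading, then despawns three seconds later.
; Overlapping anything except spawn and despawn actors adds score through SpaceGameMode and notifies charge shots via Bshot.
; A hit enemy falls with gravity and added downward velocity, then explodes after a short delay.
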(event `self.ReceiveTick`
  (params (DeltaSeconds :type "Float (single-precision)"))
  ;[1 1 1] Speed
  (if (`self.Destroyed`)
    (`PrimitiveComponent.SetEnableGravity` (`self.Base`) true)
    (`PrimitiveComponent.SetPhysicsLinearVelocity` (`self.Base`) (0.0 0.0 -50.0) true "None")
    (else
      (`PrimitiveComponent.SetPhysicsLinearVelocity` (`self.Base`) (* (`SceneComponent.GetForwardVector` (`self.Base`)) (`self.Speed`)) false "None")
      ;[1 1 1] Rotate to Equal Player
      (`SceneComponent.K2_AddWorldRotation` (`self.Base`) (`KismetMathLibrary.RInterpTo` (struct) (`KismetMathLibrary.NormalizedDeltaRotator` (`self.target`) (`SceneComponent.K2_GetComponentRotation` (`self.Base`))) (`GameplayStatics.GetWorldDeltaSeconds`) 0.5) false false))))

(event `self.ReceiveActorBeginOverlap`
  (params (OtherActor :type "Actor Object Reference"))
  ;[1 1 1] Destroy
  (cast `/Game/Blueprints/TriggerSpawn` OtherActor
    (:`CastFailed`
      (cast `/Game/Blueprints/DespawnPlayer` OtherActor
        (:`CastFailed`
          (cast `/Game/Blueprints/Despawner` OtherActor
            (:`CastFailed`
              (if (not (`self.Destroyed`))
                (set `self.Destroyed` true)
                ;[1 1 1] Add Score
                (bind _asspace_game_mode (cast `/Game/Blueprints/SpaceGameMode` (`GameplayStatics.GetGameMode`)))
                (`/Game/Blueprints/SpaceGameMode.Add Score` _asspace_game_mode 1)
                (bind _ascharge_shot_p (cast `/Game/Blueprints/Player/ChargeShotP` OtherActor)
                  (:`then`
                    (`/Game/Blueprints/Player/ChargeShotP.Bshot` _ascharge_shot_p))
                  (:`CastFailed`
                    _))
                (`KismetSystemLibrary.Delay` 1.2)
                (`GameplayStatics.SpawnEmitterAtLocation` "/Game/StarterContent/Particles/P_Explosion.P_Explosion" (`SceneComponent.K2_GetComponentLocation` (`self.Base`)) (struct) (7.0 7.0 7.0))
                (`self.K2_DestroyActor`)))))))))

(event `self.ReceiveBeginPlay`
  (set `self.target` (`SceneComponent.K2_GetComponentRotation` (`self.Base`)))
  (`KismetSystemLibrary.Delay` 8.0)
  (set `self.target` (struct :`Pitch` 90.0))
  (`KismetSystemLibrary.Delay` 3.0)
  (`self.K2_DestroyActor`))

(fn `UserConstructionScript`)