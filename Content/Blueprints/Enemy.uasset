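; Enemy actor for a space game that flies forward as a physics body and scores a point when taken down.
; Tick drives Base along its forward vector while gradually turning it to match the rotation of the player's Normal actor.
; Overlaps ignore spawn triggers and DespawnPlayer; a Despawner removes it silently.
; Other overlaps add score, notify charge shots, and make it plummet before exploding 1.2 seconds later.
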(event `self.ReceiveTick`
  (params (DeltaSeconds :type "Float (single-precision)"))
  ;[1 1 1] Speed
  (if (`self.Destroyed`)
    (`PrimitiveComponent.SetEnableGravity` (`self.Base`) true)
    (`PrimitiveComponent.SetPhysicsLinearVelocity` (`self.Base`) (0.0 0.0 -50.0) true "None")
    (else
      (`PrimitiveComponent.SetPhysicsLinearVelocity` (`self.Base`) (* (`SceneComponent.GetForwardVector` (`self.Base`)) (`self.Speed`)) false "None")
      ;[1 1 1] Rotate to Equal Player
      (`SceneComponent.K2_AddWorldRotation` (`self.Base`) (`KismetMathLibrary.RInterpTo` (struct) (`KismetMathLibrary.NormalizedDeltaRotator` (`SceneComponent.K2_GetComponentRotation` (`Actor.RootComponent` (`self.player`))) (`SceneComponent.K2_GetComponentRotation` (`self.Base`))) (`GameplayStatics.GetWorldDeltaSeconds`) 0.5) false false))))

(event `self.ReceiveActorBeginOverlap`
  (params (OtherActor :type "Actor Object Reference"))
  ;[1 1 1] Destroy
  (cast `/Game/Blueprints/TriggerSpawn` OtherActor
    (:`CastFailed`
      (cast `/Game/Blueprints/DespawnPlayer` OtherActor
        (:`CastFailed`
          (if (not (`self.Destroyed`))
            (set `self.Destroyed` true)
            (cast `/Game/Blueprints/Despawner` OtherActor
              (:`then`
                (`self.K2_DestroyActor`))
              (:`CastFailed`
                ;[1 1 1] Add Score
                (bind _asspace_game_mode (cast `/Game/Blueprints/SpaceGameMode` (`GameplayStatics.GetGameMode`)))
                (`/Game/Blueprints/SpaceGameMode.Add Score` _asspace_game_mode 1)
                (bind _ascharge_shot_p (cast `/Game/Blueprints/Player/ChargeShotP` OtherActor)
                  (:`then`
                    (`/Game/Blueprints/Player/ChargeShotP.Bshot` _ascharge_shot_p))
                  (:`CastFailed`
                    _))
                (`KismetSystemLibrary.Delay` 1.2)
                (`GameplayStatics.SpawnEmitterAtLocation` "/Game/StarterContent/Particles/P_Explosion.P_Explosion" (`SceneComponent.K2_GetComponentLocation` (`self.Base`)) (struct) (7.0 7.0 7.0))
                (`self.K2_DestroyActor`)))))))))

(event `self.ReceiveBeginPlay`
  (bind _returnvalue (`GameplayStatics.GetActorOfClass` "/Game/Blueprints/Player/Normal.Normal_C"))
  (set `self.player` _returnvalue)
  (set `self.Start rot` (`SceneComponent.K2_GetComponentRotation` (`self.Base`))))

(fn `UserConstructionScript`)